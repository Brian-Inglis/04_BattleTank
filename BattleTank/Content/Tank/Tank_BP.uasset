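; Tank Blueprint that assembles a tank from separate body, turret, barrel and track components.
; The construction script snaps the turret and right track to the Tank component and the barrel to the turret, keeping relative rotation and scale.
; The right track attach call appears twice, and no left track is attached here.
; The event graph holds only disabled placeholder events, so this graph adds no runtime behavior.
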(event EventBeginPlay)

(event Collision|EventActorBeginOverlap
  (params (OtherActor :type Actor%20Object%20Reference)))

(event EventTick
  (params (DeltaSeconds :type Float%20%28single-precision%29)))

(fn ConstructionScript
  (Transformation|AttachComponentToComponent (Variables|Default|GetBarrel) (Variables|Default|GetTurret) "None" "SnapToTarget" "KeepRelative" "KeepRelative" true)
  (Transformation|AttachComponentToComponent (Variables|Default|GetTurret) (Variables|Default|GetTank) "None" "SnapToTarget" "KeepRelative" "KeepRelative" true)
  (Transformation|AttachComponentToComponent (Variables|Default|GetRight%20Track) (Variables|Default|GetTank) "None" "SnapToTarget" "KeepRelative" "KeepRelative" true)
  (Transformation|AttachComponentToComponent (Variables|Default|GetRight%20Track) (Variables|Default|GetTank) "None" "SnapToTarget" "KeepRelative" "KeepRelative" true))